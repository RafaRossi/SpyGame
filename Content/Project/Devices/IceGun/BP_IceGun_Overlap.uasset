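; Ice gun device that toggles the frozen state of freezable objects overlapping its capsule when used.
; Capsule begin overlap adds the other actor's FrozenableComponent to a duplicate-free list.
; Use calls ChangeFrozenState on every listed component.
; End overlap looks up the component on the gun itself rather than the departing actor, so departed objects' components stay listed.
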(event OnComponentBeginOverlap(Capsule)
  (params (OverlappedComponent :type Primitive%20Component%20Object%20Reference) (OtherActor :type Actor%20Object%20Reference) (OtherComp :type Primitive%20Component%20Object%20Reference) (OtherBodyIndex :type Integer) (bFromSweep :type Boolean) (SweepResult :type Hit%20Result%20Structure%20%28by%20ref%29))
  (bind _returnvalue (Actor|GetComponentbyClass OtherActor "/Script/Spy.FrozenableComponent"))
  (bind _overlaping_frozenable_components (Variables|Variables|GetOverlaping%20Frozenable%20Components))
  (if (Utilities|IsValid _returnvalue)
    (if (not (Utilities|Array|ContainsItem _overlaping_frozenable_components _returnvalue))
      (Utilities|Array|Add _overlaping_frozenable_components _returnvalue))))

(event OnComponentEndOverlap(Capsule)
  (params (OverlappedComponent :type Primitive%20Component%20Object%20Reference) (OtherActor :type Actor%20Object%20Reference) (OtherComp :type Primitive%20Component%20Object%20Reference) (OtherBodyIndex :type Integer))
  (bind _returnvalue (Actor|GetComponentbyClass "/Script/Spy.FrozenableComponent"))
  (bind _overlaping_frozenable_components (Variables|Variables|GetOverlaping%20Frozenable%20Components))
  (if (Utilities|IsValid _returnvalue)
    (if (Utilities|Array|ContainsItem _overlaping_frozenable_components _returnvalue)
      (Utilities|Array|RemoveItem _overlaping_frozenable_components _returnvalue))))

(event EventUse
  (for _array_element (Variables|Variables|GetOverlaping%20Frozenable%20Components)
    (Class|FrozenableComponent|ChangeFrozenState _array_element)))

(fn ConstructionScript)