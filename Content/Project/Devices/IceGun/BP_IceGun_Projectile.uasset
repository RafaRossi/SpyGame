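; Projectile variant of the ice gun device, which keeps at most one object frozen at a time.
; Use spawns a BP_IceProjectile at the spawn point and binds to its OnFrozen event.
; HandleCurrentFrozenObject unfreezes the object held in a soft reference, then freezes and stores the new component.
; Passing the already frozen component again only unfreezes it and clears the reference, acting as a toggle.
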(event EventUse
  (bind _projectile_spawn_point (Variables|Default|GetProjectile%20Spawn%20Point))
  (bind _returnvalue (Game|SpawnActorfromClass "/Game/Project/Devices/IceGun/BP_IceProjectile.BP_IceProjectile_C" (Math|Transform|MakeTransform (Transformation|GetWorldLocation _projectile_spawn_point) (Transformation|GetWorldRotation _projectile_spawn_point)) "Undefined" "MultiplyWithRoot" 0 0))
  (EventDispatchers|BindEventtoOnFrozen _returnvalue (EventDispatchers|CreateEvent :!event HandleCurrentFrozenObject)))

(fn ConstructionScript)

(fn HandleCurrentFrozenObject
  (params (Frozenable%20Component :type Frozenable%20Component%20Object%20Reference))
  (Utilities|FlowControl|Sequence
    (:then_0
      (if (Utilities|IsValidSoftObjectReference (Variables|Default|GetCurrent%20Frozen%20Object))
        (Class|FrozenableComponent|Unfrozen (Utilities|ResolveSoftReference (Variables|Default|GetCurrent%20Frozen%20Object)))))
    (:then_1
      (if (!= (Utilities|ResolveSoftReference (Variables|Default|GetCurrent%20Frozen%20Object)) Frozenable%20Component)
        (Class|FrozenableComponent|Frozen Frozenable%20Component)
        (Variables|Default|SetCurrent%20Frozen%20Object (Utilities|ResolveSoftReference Frozenable%20Component))
        (else
          (Variables|Default|SetCurrent%20Frozen%20Object 0))))))