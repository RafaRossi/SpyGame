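; BP_InteractableArea is an overlap area that tracks which actors with an InteractionComponent are currently within interaction range.
; On begin overlap it prints a debug string and adds the other actor's InteractionComponent, if valid, to the OnRangeInteraction collection.
; On end overlap it removes that component if the collection contains it.
; The Blueprint only maintains this collection and triggers no interaction itself.
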(event Collision|EventActorBeginOverlap
  (params (OtherActor :type Actor%20Object%20Reference))
  (bind _returnvalue (Actor|GetComponentbyClass OtherActor "/Script/Spy.InteractionComponent"))
  (Development|PrintString "Hiii")
  (Utilities|IsValid _returnvalue
    (:Is%20Valid
      (Utilities|Array|Add (Variables|Default|GetOn%20Range%20Interaction) _returnvalue))))

(event Collision|EventActorEndOverlap
  (params (OtherActor :type Actor%20Object%20Reference))
  (bind _returnvalue (Actor|GetComponentbyClass OtherActor "/Script/Spy.InteractionComponent"))
  (bind _on_range_interaction (Variables|Default|GetOn%20Range%20Interaction))
  (Utilities|IsValid _returnvalue
    (:Is%20Valid
      (if (Utilities|Array|ContainsItem _on_range_interaction _returnvalue)
        (Utilities|Array|RemoveItem _on_range_interaction _returnvalue)))))

(fn ConstructionScript)